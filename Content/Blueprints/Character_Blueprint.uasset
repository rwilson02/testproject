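; Character Blueprint that positions an actor every frame from X and Y values scaled by a Speed variable.
; Tick enables input from player controller 0, then sets the relative location to those values times Speed and delta seconds, with Z at zero and no sweep.
; The product replaces the location instead of adding an offset to it.
; A MoveForward call is left unconnected, and the construction script is empty.
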(event EventBeginPlay)

(event Collision|EventActorBeginOverlap
  (params (OtherActor :type Actor%20Object%20Reference)))

(event EventTick
  (params (DeltaSeconds :type Float%20%28single-precision%29))
  (Input|EnableInput (Game|GetPlayerController 0))
  (Transformation|SetActorRelativeLocation (Math|Vector|MakeVector (* DeltaSeconds (* (Variables|Default|GetSpeed) (Input|AxisValues|GetX))) (* DeltaSeconds (* (Input|AxisValues|GetY) (Variables|Default|GetSpeed))) 0.0)))

(fn ConstructionScript)