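; A player pawn whose Sphere component is pushed vertically with mouse clicks.
; On BeginPlay it makes player controller 0 possess it and enables input.
; Left and right click call Impulse, which uses AddForce to apply the Force variable along world up, downward for left and upward for right.
; Each call also prints a debug string with the direction flag.
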(event EventBeginPlay
  (bind _returnvalue (Game|GetPlayerController 0))
  (Pawn|Possess _returnvalue self)
  (Input|EnableInput _returnvalue))

(event Collision|EventActorBeginOverlap
  (params (OtherActor :type Actor%20Object%20Reference)))

(event EventTick
  (params (DeltaSeconds :type Float%20%28single-precision%29)))

(event Input|ActionEvents|InputActionLeftClick
  (params (Key :type Key%20Structure :default "None"))
  (:Pressed
    (CallFunction|Impulse (Variables|Default|GetForce) false)))

(event Input|ActionEvents|InputActionRightClick
  (params (Key :type Key%20Structure :default "None"))
  (:Pressed
    (CallFunction|Impulse (Variables|Default|GetForce) true)))

(fn ConstructionScript)

(fn Impulse
  (params (Force :type Float%20%28single-precision%29) (Toward :type Boolean))
  (bind _returnvalue (Math|Vector|VectorUp))
  (bind _sphere (Variables|Default|GetSphere))
  (bind _returnvalue_2 (* _returnvalue Force))
  (if Toward
    (Physics|AddForce _sphere _returnvalue_2 "None" false)
    (else
      (Physics|AddForce _sphere (Math|Vector|NegateVector _returnvalue_2) "None" false)))
  (Development|PrintString (Class|KismetStringLibrary|BuildStringBool "penis " "" Toward)))